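; BP_PigeonGameInstance is a game instance that handles looping music that persists across level transitions.
; PlayMusic spawns a 2D sound without auto-destroy, stores its audio component and binds the finished event to LoopMusic, which restarts playback from the beginning.
; SetMusic handles replacement of the stored Music component, with a destroy call and reassignment.
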(event `PlayMusic`
  (params (Sound :type "SoundBase Object Reference"))
  (bind _returnvalue (`GameplayStatics.SpawnSound2D` Sound 1.0 1.0 0.0 null true false))
  (bind _output_get (set `self.Music` _returnvalue))
  (add `AudioComponent.OnAudioFinished` _output_get (delegate `LoopMusic`)))

(event `LoopMusic`
  (`AudioComponent.Play` (`self.Music`) 0.0))

(fn `SetMusic`
  (params (music :type "AudioComponent Object Reference"))
  (if (!= (`self.Music`) null)
    (`ActorComponent.K2_DestroyComponent` (`self.Music`)))
  (set `self.Music` music))