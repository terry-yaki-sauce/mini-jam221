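; Stick is an actor that a Pigeon can pick up and drop with the E key.
; Its Box overlap events track whether a Pigeon is in range, with begin overlap enabling player 0 input on the stick.
; E checks the PigeonBox tag and overlap flag, then toggles BeingCarried and calls StickPickUp or StickDrop on the Pigeon.
; Input stays enabled after overlap ends, and debug strings print state changes.
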(event `self.Box.OnComponentBeginOverlap`
  (params (OverlappedComponent :type "PrimitiveComponent Object Reference") (OtherActor :type "Actor Object Reference") (OtherComp :type "PrimitiveComponent Object Reference") (OtherBodyIndex :type Integer) (bFromSweep :type Boolean) (SweepResult :type "HitResult Structure (by ref)"))
  (bind _aspigeon (cast `/Game/Blueprints/Pigeon` OtherActor))
  (if (not (`ActorComponent.ComponentHasTag` (`/Game/Blueprints/Pigeon.PigeonBox` _aspigeon) "PigeonBox"))
    (`KismetSystemLibrary.PrintString` "No initial pigeon box"))
  (bind _output_get (set `self.IsOverlap` true))
  (`KismetSystemLibrary.PrintString` (`KismetStringLibrary.Conv_BoolToString` _output_get))
  (`self.EnableInput` (`GameplayStatics.GetPlayerController` 0)))

(event `self.Box.OnComponentEndOverlap`
  (params (OverlappedComponent :type "PrimitiveComponent Object Reference") (OtherActor :type "Actor Object Reference") (OtherComp :type "PrimitiveComponent Object Reference") (OtherBodyIndex :type Integer))
  (bind _aspigeon (cast `/Game/Blueprints/Pigeon` OtherActor))
  (if (`ActorComponent.ComponentHasTag` (`/Game/Blueprints/Pigeon.PigeonBox` _aspigeon) "PigeonBox")
    _
    (else
      _))
  (bind _output_get (set `self.IsOverlap` false))
  (`KismetSystemLibrary.PrintString` (`KismetStringLibrary.Conv_BoolToString` _output_get)))

(event `Key|E`
  (params (Key :type "Key Structure"))
  (:`Pressed`
    (bind _aspigeon (cast `/Game/Blueprints/Pigeon` (stale `self.Box.OnComponentBeginOverlap` OtherActor)))
    (if (`ActorComponent.ComponentHasTag` (`/Game/Blueprints/Pigeon.PigeonBox` _aspigeon) "PigeonBox")
      (if (`self.IsOverlap`)
        (if (`self.BeingCarried`)
          (bind _output_get (set `self.BeingCarried` false))
          (`KismetSystemLibrary.PrintString` (`KismetStringLibrary.Conv_BoolToString` _output_get) true true (struct :`R` 0.759733 :`G` 1.0 :`B` 0.20884 :`A` 1.0))
          (`/Game/Blueprints/Pigeon.StickDrop` _aspigeon self)
          (else
            (bind _output_get_2 (set `self.BeingCarried` true))
            (`KismetSystemLibrary.PrintString` (`KismetStringLibrary.Conv_BoolToString` _output_get_2) true true (struct :`R` 0.759733 :`G` 1.0 :`B` 0.20884 :`A` 1.0))
            (`/Game/Blueprints/Pigeon.StickPickUp` _aspigeon self))))
      (else
        (`KismetSystemLibrary.PrintString` "No pigeon box detected")))))

(fn `UserConstructionScript`)