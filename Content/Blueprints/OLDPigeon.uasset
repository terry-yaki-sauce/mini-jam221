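; OLDPigeon is a player-controlled pigeon Character that can walk and fly.
; Enhanced Input actions drive Move and Look, moving along the control rotation's right and forward vectors and turning the controller's yaw and pitch.
; BeginFly and EndFly switch CharacterMovement between Flying and Walking and set IsFlying, which makes Tick add constant upward input scaled by FlySpeed.
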(event `self.ReceiveTick`
  (params (DeltaSeconds :type "Float (single-precision)"))
  (if (`self.isFlying`)
    (`self.AddMovementInput` (0.0 0.0 1.0) (`self.FlySpeed`))))

(event `EnhancedInput|/Game/Input/Actions/IA_Move`
  (params (ActionValue :type "Vector2D Structure") (ElapsedSeconds :type "Float (double-precision)") (TriggeredSeconds :type "Float (double-precision)") (InputAction :type "InputAction Object Reference" :default "/Game/Input/Actions/IA_Move.IA_Move"))
  (bind (_x _y) (`KismetMathLibrary.BreakVector2D` ActionValue))
  (:`Triggered`
    (`self.Move` _x _y)))

(event `EnhancedInput|/Game/Input/Actions/IA_Look`
  (params (ActionValue :type "Vector2D Structure") (ElapsedSeconds :type "Float (double-precision)") (TriggeredSeconds :type "Float (double-precision)") (InputAction :type "InputAction Object Reference" :default "/Game/Input/Actions/IA_Look.IA_Look"))
  (bind (_x _y) (`KismetMathLibrary.BreakVector2D` ActionValue))
  (:`Triggered`
    (`self.Look` _x _y)))

(event `EnhancedInput|/Game/Input/Actions/IA_BeginFly`
  (params (ActionValue :type Boolean) (ElapsedSeconds :type "Float (double-precision)") (TriggeredSeconds :type "Float (double-precision)") (InputAction :type "InputAction Object Reference" :default "/Game/Input/Actions/IA_BeginFly.IA_BeginFly"))
  (:`Triggered`
    (`self.BeginFly`)))

(event `EnhancedInput|/Game/Input/Actions/IA_EndFly`
  (params (ActionValue :type Boolean) (ElapsedSeconds :type "Float (double-precision)") (TriggeredSeconds :type "Float (double-precision)") (InputAction :type "InputAction Object Reference" :default "/Game/Input/Actions/IA_EndFly.IA_EndFly"))
  (:`Triggered`
    (`self.EndFly`)))

(fn `BeginFly`
  (`CharacterMovementComponent.SetMovementMode` (`self.CharacterMovement`) "MOVE_Flying" 0)
  (set `self.isFlying` true))

(fn `EndFly`
  (`CharacterMovementComponent.SetMovementMode` (`self.CharacterMovement`) "MOVE_Walking" 0)
  (set `self.isFlying` false))

(fn `Look`
  (params (X :type "Float (double-precision)") (Y :type "Float (double-precision)"))
  (`self.AddControllerYawInput` X)
  (`self.AddControllerPitchInput` Y))

(fn `Move`
  (params (X :type "Float (double-precision)") (Y :type "Float (double-precision)"))
  (`self.AddMovementInput` (`KismetMathLibrary.GetRightVector` (`self.GetControlRotation`)) X)
  (`self.AddMovementInput` (`KismetMathLibrary.GetForwardVector` (`self.GetControlRotation`)) Y))

(fn `UserConstructionScript`)