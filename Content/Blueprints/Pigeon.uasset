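; Player pigeon character that walks, flies and carries sticks in its mouth for a nest-building game.
; Enhanced Input drives camera-relative movement, climbing flight and stick pickup or drop, refusing sticks already in the nest.
; Tick selects Idle, Walk or Fly states that play procedural mesh Timelines, and smoothly turns the grounded bird.
; BeginPlay creates the objective and pause widgets, with pause visibility driven by a GS_Pigeon game state event.
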(event `self.ReceiveTick`
  (params (DeltaSeconds :type "Float (single-precision)"))
  (`|ExecutionSequence`
    (:`then_0`
      ; Flight
      (if (`self.isFlying`)
        (`self.AddMovementInput` (0.0 0.0 1.0) (`self.FlySpeed`))))
    (:`then_1`
      ; Animation State
      (if (`self.InAir`)
        (`self.SetAnimationState` "NewEnumerator2")
        (elif (< (`KismetMathLibrary.VSize` (`self.GetVelocity`)) 0.1)
          (`self.SetAnimationState` "NewEnumerator0")
          (else
            (`self.SetAnimationState` "NewEnumerator1")))))
    (:`then_2`
      (if (not (`self.InAir`))
        (`self.K2_SetActorRotation` (`KismetMathLibrary.RInterpTo` (`self.K2_GetActorRotation`) (`self.TargetZDir`) DeltaSeconds 10.0))))))

(event `OnPauseChanged`
  (params (paused :type Boolean))
  ; Pausing
  (`Widget.SetVisibility` (`self.PauseWidget`) (select `bool` paused :`false` (enumliteral `ESlateVisibility` "Hidden") :`true` (enumliteral `ESlateVisibility` "Visible"))))

(event `StickPickUp`
  (params (Actor :type "Actor Object Reference"))
  ; Stick Functions
  (bind _asstick (cast `/Game/Blueprints/Stick` Actor))
  (`self.K2_AttachToComponent` Actor (`self.Head`) "Mouth" "SnapToTarget" "SnapToTarget" "SnapToTarget" true)
  (set `self.HoldingStick` true)
  (set `self.StickRef` _asstick))

(event `EnhancedInput|/Game/Input/Actions/IA_Move`
  (params (ActionValue :type "Vector2D Structure") (ElapsedSeconds :type "Float (double-precision)") (TriggeredSeconds :type "Float (double-precision)") (InputAction :type "InputAction Object Reference" :default "/Game/Input/Actions/IA_Move.IA_Move"))
  (bind (_x _y) (`KismetMathLibrary.BreakVector2D` ActionValue))
  ; Movement
  (:`Triggered`
    (`self.Move` _x _y)))

(event `StickDrop`
  (params (Actor :type "Actor Object Reference"))
  ; Stick Functions
  (`self.K2_DetachFromActor` Actor "KeepWorld" "KeepWorld" "KeepWorld")
  (`self.K2_SetActorLocation` Actor (`KismetMathLibrary.MakeVector` (.x (`self.K2_GetActorLocation` Actor)) (.y (`self.K2_GetActorLocation` Actor)) 1.0) false false)
  (set `self.HoldingStick` false)
  (set `self.StickRef` null))

(event `EnhancedInput|/Game/Input/Actions/IA_Pause`
  (params (ActionValue :type Boolean) (ElapsedSeconds :type "Float (double-precision)") (TriggeredSeconds :type "Float (double-precision)") (InputAction :type "InputAction Object Reference" :default "/Game/Input/Actions/IA_Pause.IA_Pause"))
  ; Pausing
  (:`Triggered`
    (message `/Game/Game/BPI_GS.Pause` (`GameplayStatics.GetGameState`))))

(event `EnhancedInput|/Game/Input/Actions/IA_Look`
  (params (ActionValue :type "Vector2D Structure") (ElapsedSeconds :type "Float (double-precision)") (TriggeredSeconds :type "Float (double-precision)") (InputAction :type "InputAction Object Reference" :default "/Game/Input/Actions/IA_Look.IA_Look"))
  (bind (_x _y) (`KismetMathLibrary.BreakVector2D` ActionValue))
  ; Movement
  (:`Triggered`
    (`self.Look` _x _y)))

(event `EnhancedInput|/Game/Input/Actions/IA_BeginFly`
  (params (ActionValue :type Boolean) (ElapsedSeconds :type "Float (double-precision)") (TriggeredSeconds :type "Float (double-precision)") (InputAction :type "InputAction Object Reference" :default "/Game/Input/Actions/IA_BeginFly.IA_BeginFly"))
  ; Movement
  (:`Triggered`
    (`self.BeginFly`)))

(event `EnhancedInput|/Game/Input/Actions/IA_Interact`
  (params (ActionValue :type Boolean) (ElapsedSeconds :type "Float (double-precision)") (TriggeredSeconds :type "Float (double-precision)") (InputAction :type "InputAction Object Reference" :default "/Game/Input/Actions/IA_Interact.IA_Interact"))
  ; IA Baed Interaction
  (:`Triggered`
    (if (not (`self.HoldingStick`))
      (if (!= (`self.InteractionTarget`) null)
        (bind _value (`/Game/Blueprints/Stick.isInNest` (`self.InteractionTarget`)))
        (if (not _value)
          (`PrimitiveComponent.SetSimulatePhysics` (`/Game/Blueprints/Stick.Stick mesh` (`self.InteractionTarget`)) false)
          (`self.K2_AttachToComponent` (`self.InteractionTarget`) (`self.Head`) "Mouth" "SnapToTarget" "SnapToTarget" "KeepWorld" true)
          (set `self.HoldingStick` true)
          (set `self.StickRef` (`self.InteractionTarget`))
          (set `self.InteractionTarget` null)))
      (elif (!= (`self.StickRef`) null)
        (if (`PrimitiveComponent.IsOverlappingComponent` (`/Game/Blueprints/Stick.Box` (`self.StickRef`)) (`self.PigeonBox`))
          (`self.K2_DetachFromActor` (`self.StickRef`) "KeepWorld" "KeepWorld" "KeepWorld")
          (`PrimitiveComponent.SetSimulatePhysics` (`/Game/Blueprints/Stick.Stick mesh` (`self.StickRef`)) true)
          (set `self.HoldingStick` false)
          (set `self.StickRef` null))
        (else
          (`KismetSystemLibrary.PrintString` "Holding a Null Stick?"))))))

(event `EnhancedInput|/Game/Input/Actions/IA_EndFly`
  (params (ActionValue :type Boolean) (ElapsedSeconds :type "Float (double-precision)") (TriggeredSeconds :type "Float (double-precision)") (InputAction :type "InputAction Object Reference" :default "/Game/Input/Actions/IA_EndFly.IA_EndFly"))
  ; Movement
  (:`Triggered`
    (`self.EndFly`)))

(event `self.ReceiveBeginPlay`
  (`|ExecutionSequence`
    (:`then_0`
      (`self.InitAnimationTransforms`))
    (:`then_1`
      (`self.SetAnimationState` "NewEnumerator0"))
    (:`then_2`
      (`|ExecutionSequence`
        (:`then_0`
          ; UI Init
          (bind _asplayer_controller (cast `PlayerController` (`self.GetController`)))
          (bind _returnvalue (`|CreateWidget` "/Game/UI/UI.UI_C" _asplayer_controller))
          (`UserWidget.AddToViewport` _returnvalue 0)
          (`TextBlock.SetText` (`/Game/UI/UI.TextBlock_65` _returnvalue) "Collect ten sticks to build a nest! Make sure your egg is warm, but not too warm!"))
        (:`then_1`
          (bind _returnvalue_2 (`|CreateWidget` "/Game/UI/PauseMenu.PauseMenu_C" _asplayer_controller))
          (bind _output_get (set `self.PauseWidget` _returnvalue_2))
          (`Widget.SetVisibility` _returnvalue_2 "Hidden")
          (`Widget.SetVisibility` _output_get "Hidden")
          (`UserWidget.AddToViewport` _returnvalue_2 0)
          (`UserWidget.AddToViewport` _output_get 0))))
    (:`then_3`
      (bind _asgs_pigeon (cast `/Game/Game/GS_Pigeon` (`GameplayStatics.GetGameState`)))
      (add `/Game/Game/GS_Pigeon.OnPauseChanged` _asgs_pigeon (`|CreateDelegate` :!event `OnPauseChanged`)))))

(fn `BeginFly`
  (`CharacterMovementComponent.SetMovementMode` (`self.CharacterMovement`) "MOVE_Flying" 0)
  (set `self.isFlying` true))

(fn `EndFly`
  (`CharacterMovementComponent.SetMovementMode` (`self.CharacterMovement`) "MOVE_Falling" 0)
  (set `self.isFlying` false))

(fn `InitAnimationTransforms`
  (`|ExecutionSequence`
    (:`then_0`
      (set `self.InitialMeshLocation` (`SceneComponent.RelativeLocation` (`self.Mesh`))))
    (:`then_1`
      (set `self.InitialHeadLocation` (`SceneComponent.RelativeLocation` (`self.Head`))))
    (:`then_2`
      (set `self.InitialMeshRelativeRotation` (`SceneComponent.RelativeRotation` (`self.Mesh`))))
    (:`then_3`
      (set `self.TargetZDir` (`self.K2_GetActorRotation`)))))

(fn `Look`
  (params (X :type "Float (double-precision)") (Y :type "Float (double-precision)"))
  (`self.AddControllerYawInput` X)
  (`self.AddControllerPitchInput` Y))

(fn `Move`
  (params (X :type "Float (double-precision)") (Y :type "Float (double-precision)"))
  (bind (_returnvalue_roll _returnvalue_pitch _returnvalue_yaw) (`KismetMathLibrary.BreakRotator` (`self.GetControlRotation`)))
  (bind (_returnvalue_roll_2 _returnvalue_pitch_2 _returnvalue_yaw_2) (`KismetMathLibrary.BreakRotator` (`self.GetControlRotation`)))
  (bind _returnvalue (`KismetMathLibrary.GetForwardVector` (`KismetMathLibrary.MakeRotator` 0.0 0.0 _returnvalue_yaw_2)))
  (bind _returnvalue_2 (`KismetMathLibrary.GetRightVector` (`KismetMathLibrary.MakeRotator` _returnvalue_roll 0.0 _returnvalue_yaw)))
  (bind (_returnvalue_roll_3 _returnvalue_pitch_3 _returnvalue_yaw_3) (`KismetMathLibrary.BreakRotator` (`KismetMathLibrary.Conv_VectorToRotator` (+ (* _returnvalue Y) (* _returnvalue_2 X)))))
  (`self.AddMovementInput` _returnvalue_2 (select `bool` (`self.isFlying`) :`false` X :`true` (* X (`self.FlySpeed`))))
  (`self.AddMovementInput` _returnvalue (select `bool` (`self.isFlying`) :`false` Y :`true` (* Y (`self.FlySpeed`))))
  (set `self.TargetZDir` (`KismetMathLibrary.MakeRotator` (.roll (`self.K2_GetActorRotation`)) (.pitch (`self.K2_GetActorRotation`)) _returnvalue_yaw_3)))

(fn `SetAnimationState`
  (params (state :type "/Game/Blueprints/PigeonState Enum" :default "NewEnumerator0"))
  (switch `/Game/Blueprints/PigeonState` state
    (:`NewEnumerator0`
      (if (not (`|EnumEquality` (`self.CurrentAnimationState`) "NewEnumerator0"))
        (set `self.CurrentAnimationState` "NewEnumerator0")
        (`self.StopAnimationTimelines`)
        (`TimelineComponent.PlayFromStart` (`self.IdleTimeline`))))
    (:`NewEnumerator1`
      (if (not (`|EnumEquality` (`self.CurrentAnimationState`) "NewEnumerator1"))
        (set `self.CurrentAnimationState` "NewEnumerator1")
        (`self.StopAnimationTimelines`)
        (`TimelineComponent.PlayFromStart` (`self.Walk TImeline`))))
    (:`NewEnumerator2`
      (if (not (`|EnumEquality` (`self.CurrentAnimationState`) "NewEnumerator2"))
        (set `self.CurrentAnimationState` "NewEnumerator2")
        (`self.StopAnimationTimelines`)
        (`TimelineComponent.PlayFromStart` (`self.Fly Timeline`))))))

(fn `StopAnimationTimelines`
  (`self.StopIdleTimeline`)
  (`self.StopWalkTimeline`)
  (`self.StopFlyTimeline`))

(fn `StopFlyTimeline`
  (`TimelineComponent.Stop` (`self.Fly Timeline`)))

(fn `StopIdleTimeline`
  (`TimelineComponent.Stop` (`self.IdleTimeline`)))

(fn `StopWalkTimeline`
  (`TimelineComponent.Stop` (`self.Walk TImeline`))
  (`SceneComponent.K2_SetRelativeRotation` (`self.Mesh`) (`self.InitialMeshRelativeRotation`) false false)
  (`SceneComponent.K2_SetRelativeLocation` (`self.Mesh`) (`self.InitialMeshLocation`) false false))

(fn `TrySetInteractionTarget`
  (params (Stick :type "/Game/Blueprints/Stick Object Reference"))
  (if (not (`self.HoldingStick`))
    (set `self.InteractionTarget` Stick)))

(fn `UserConstructionScript`)