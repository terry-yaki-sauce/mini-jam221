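; Nest is the pigeon's goal actor that counts sticks inside it and ends the game in a win once enough are gathered.
; Box overlaps raise or lower the count and set each Stick's InNest flag, with entering sticks also having their input disabled.
; A NestWidg created at BeginPlay shows the count, refreshed every Tick.
; Tick also checks for ten sticks, then shows WinLoseScreen and pauses the game.
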(event `self.ReceiveTick`
  (params (DeltaSeconds :type "Float (single-precision)"))
  (bind _numofsticks (`self.NumOfSticks`))
  (`TextBlock.SetText` (`/Game/Blueprints/Widget/NestWidg.NumOfSticks` (stale `self.ReceiveBeginPlay` _returnvalue)) (`KismetTextLibrary.Conv_IntToText` _numofsticks))
  (if (>= _numofsticks 10)
    (bind _returnvalue (`|CreateWidget` "/Game/Blueprints/Widget/Win-LoseScreen.Win-LoseScreen_C"))
    (`TextBlock.SetText` (`/Game/Blueprints/Widget/Win-LoseScreen.WinLose` _returnvalue) "You Win!!!")
    (`UserWidget.AddToViewport` _returnvalue 0)
    (`GameplayStatics.SetGamePaused` true)))

(event `self.ReceiveBeginPlay`
  (bind _returnvalue (`|CreateWidget` "/Game/Blueprints/Widget/NestWidg.NestWidg_C" (`GameplayStatics.GetPlayerController` 0)))
  (`UserWidget.AddToViewport` _returnvalue 0))

(event `self.Box.OnComponentBeginOverlap`
  (params (OverlappedComponent :type "PrimitiveComponent Object Reference") (OtherActor :type "Actor Object Reference") (OtherComp :type "PrimitiveComponent Object Reference") (OtherBodyIndex :type Integer) (bFromSweep :type Boolean) (SweepResult :type "HitResult Structure (by ref)"))
  (bind _asstick (cast `/Game/Blueprints/Stick` OtherActor))
  (`/Engine/EditorBlueprintResources/StandardMacros.IncrementInt` (`self.NumOfSticks`)
    (:`  `
      (set `/Game/Blueprints/Stick.InNest` true _asstick)
      (`self.DisableInput` _asstick (`GameplayStatics.GetPlayerController` 0)))))

(event `self.Box.OnComponentEndOverlap`
  (params (OverlappedComponent :type "PrimitiveComponent Object Reference") (OtherActor :type "Actor Object Reference") (OtherComp :type "PrimitiveComponent Object Reference") (OtherBodyIndex :type Integer))
  (bind _asstick (cast `/Game/Blueprints/Stick` OtherActor))
  (`/Engine/EditorBlueprintResources/StandardMacros.DecrementInt` (`self.NumOfSticks`)
    (:`  `
      (set `/Game/Blueprints/Stick.InNest` false _asstick))))

(fn `UserConstructionScript`)